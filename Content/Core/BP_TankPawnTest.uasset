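; BP_TankPawnTest is a pawn Blueprint that handles player input for interaction, the quest list and saving.
; The Interaction action calls both Interact and Collect on its InteractionComponent, and the quest action toggles quest list visibility.
; Two save inputs each set global time dilation to zero and open a widget, either W_Saving or W_New_Saving.
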(event EventBeginPlay)

(event Collision|EventActorBeginOverlap
  (params (OtherActor :type Actor%20Object%20Reference)))

(event EventTick
  (params (DeltaSeconds :type Float%20%28single-precision%29)))

(event Input|ActionEvents|InputActionInteraction
  (params (Key :type Key%20Structure :default "None"))
  (:Pressed
    (Class|InteractionComponent|Interact (Variables|Default|GetInteractionComponent))
    (Class|InteractionComponent|Collect (Variables|Default|GetInteractionComponent))))

(event Input|ActionEvents|InputActionQuestsButton
  (params (Key :type Key%20Structure :default "None"))
  (:Pressed
    (Class|TankPawn|ToggleQuestListVisibility)))

(event Input|ActionEvents|InputActionSaveMenu
  (params (Key :type Key%20Structure :default "None"))
  (:Pressed
    (Utilities|Time|SetGlobalTimeDilation 0.0)
    (bind _returnvalue (UserInterface|CreateWidget "/Game/Widgets/W_Saving.W_Saving_C" (Game|GetPlayerController 0)))
    (UserInterface|Viewport|AddtoViewport _returnvalue 0)))

(event Input|ActionEvents|InputActionNewSaveMenu
  (params (Key :type Key%20Structure :default "None"))
  (:Pressed
    (Utilities|Time|SetGlobalTimeDilation 0.0)
    (bind _returnvalue (UserInterface|CreateWidget "/Game/Widgets/W_New_Saving.W_New_Saving_C" (Game|GetPlayerController 0)))
    (UserInterface|Viewport|AddtoViewport _returnvalue 0)))

(fn ConstructionScript)